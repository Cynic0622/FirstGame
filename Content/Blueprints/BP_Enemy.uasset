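; BP_Enemy is a melee enemy that chases the player and reports its death to BP_WaveSpawner.
; The Wonder event loops AIMoveTo and a push montage while the player lives, retrying failed moves.
; A montage notify sphere-traces from AttackTracePos through the player and applies damage to the hit actor.
; Taking damage knocks it away from the player; at zero health it ragdolls, is destroyed after a delay and triggers CheckForEnemies.
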(event `self.ReceiveBeginPlay`
  (`self.Wonder`))

(event `Wonder`
  (bind _returnvalue (`SceneComponent.K2_GetComponentLocation` (`self.Attack Trace Pos`)))
  ;[1 1 1] Chase Player
  (`|AIMoveTo` self (0.0 0.0 0.0) (`GameplayStatics.GetPlayerCharacter` 0)
    (:`OnSuccess`
      (if (`self.Can Attack`)
        (`|PlayMontage` (`self.Mesh`) "/Game/Characters/Mannequins/Animations/Manny/Push_Montage.Push_Montage"
          (:`then`
            (set `self.Can Attack` false))
          (:`OnCompleted`
            (bind _outactors (`GameplayStatics.GetAllActorsOfClass` "/Game/Blueprints/BP_Player.BP_Player_C"))
            (bind _output_get (set `self.PlayerRef` (`|GetArrayItem` _outactors)))
            (if (<= (`/Game/Blueprints/BP_Player.Health` _output_get) 0.0)
              (set `self.Can Attack` false)
              (else
                (set `self.Can Attack` true)
                (`self.Wonder`))))
          (:`OnNotifyBegin`
            (bind _outactors_2 (`GameplayStatics.GetAllActorsOfClass` "/Game/Blueprints/BP_Player.BP_Player_C"))
            (bind _output_get_2 (set `self.Enemy` (`|GetArrayItem` _outactors_2)))
            (bind _outhit (`KismetSystemLibrary.SphereTraceSingleForObjects` :`Start` _returnvalue :`End` (+ (* (- (`self.K2_GetActorLocation` _output_get_2) _returnvalue) 2.0) _returnvalue) :`Radius` 25.0 :`ObjectTypes` (`|MakeArray` "ObjectTypeQuery3" :!type "EObjectTypeQuery Enum") :`DrawDebugType` "ForDuration"))
            (`GameplayStatics.ApplyDamage` (`.HitActor` (`GameplayStatics.BreakHitResult` _outhit)) 10.0)))))
    (:`OnFail`
      (`self.Wonder`))))

(event `self.ReceiveAnyDamage`
  (params (Damage :type "Float (single-precision)") (DamageType :type "DamageType Object Reference") (InstigatedBy :type "Controller Object Reference") (DamageCauser :type "Actor Object Reference"))
  ;[1 1 1] Damage
  (set `self.Health` (- (`self.Health`) Damage))
  (if (<= (`self.Health`) 0.0)
    (`PrimitiveComponent.SetSimulatePhysics` (`self.Mesh`) true)
    (set `self.Can Attack` false)
    (`CharacterMovementComponent.DisableMovement` (`self.CharacterMovement`))
    (`KismetSystemLibrary.Delay` 3.0)
    (`self.K2_DestroyActor`)
    (bind _returnvalue (`GameplayStatics.GetActorOfClass` "/Game/Blueprints/BP_WaveSpawner.BP_WaveSpawner_C"))
    (`/Game/Blueprints/BP_WaveSpawner.Check For Enemies` _returnvalue)
    (else
      (bind _outactors (`GameplayStatics.GetAllActorsOfClass` "/Game/Blueprints/BP_Player.BP_Player_C"))
      (bind _output_get (set `self.AttackRef` (`|GetArrayItem` _outactors)))
      (`self.LaunchCharacter` (* (- (`self.K2_GetActorLocation`) (`self.K2_GetActorLocation` _output_get)) 10.0)))))

(fn `UserConstructionScript`)